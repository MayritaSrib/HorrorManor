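; BP_AI is an enemy AI pawn that detects players and performs a melee attack.
; PawnSensing sets the Blackboard "SeenPlayer?" key when it sees a Player-tagged pawn, while a looping half-second timer clears it.
; AttackPlayer plays a montage and immediately sphere-traces forward from AttackTracePoint for pawns, damaging any hit.
; The Attacking flag blocks repeat attacks until the montage completes.
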(event OnSeePawn(PawnSensing)
  (params (Pawn :type Pawn%20Object%20Reference))
  ;[0.15 0.15 0.15 0.5] Logic for finding player
  (if (Actor|ActorHasTag Pawn "Player")
    (AI|Components|Blackboard|SetValueasBool (AI|GetBlackboard (AI|GetAIController self)) (Utilities|Name|MakeLiteralName "SeenPlayer?") true) ; AI Seen Player
  ))

(event Custom|Attack%20Player
  (bind _attack_trace_point (Variables|Default|GetAttack%20Trace%20Point))
  (bind _returnvalue (Transformation|GetWorldLocation _attack_trace_point))
  ;[0.15 0.15 0.15 0.5] Attack Player Logic
  (if (not (Variables|Default|Getattacking?))
    (Variables|Default|Setattacking? true)
    (Animation|Montage|PlayMontage (Variables|Character|GetMesh) "/Game/AI/AM_AttackPlayer.AM_AttackPlayer"
      (:then
        ;[0.15 0.15 0.15 0.5] Logic to create a sphere around the player to apply damage
        (bind (_outhit _returnvalue_2) (Collision|SphereTraceForObjects _returnvalue (+ _returnvalue (* (Math|Vector|GetForwardVector (Transformation|GetWorldRotation _attack_trace_point)) 7e+01)) 25.0 (Utilities|Array|MakeArray "ObjectTypeQuery3") false 0 "None"))
        (if _returnvalue_2
          (Game|Damage|ApplyDamage (.HitActor (Collision|BreakHitResult _outhit)) 1e+01 0 0)))
      (:OnCompleted
        (Variables|Default|Setattacking? false)))))

(event Custom|StopSeeingPlayer
  ;[0.15 0.15 0.15 0.5] Enable Player Sensing to break loop
  (AI|Components|Blackboard|SetValueasBool (AI|GetBlackboard (AI|GetAIController self)) (Utilities|Name|MakeLiteralName "SeenPlayer?") false) ; AI Seen Player
)

(event EventBeginPlay
  ;[0.15 0.15 0.15 0.5] Enable Player Sensing to break loop
  (Utilities|Time|SetTimerbyEvent (delegate Custom|StopSeeingPlayer) 0.5 true))

(fn ConstructionScript)